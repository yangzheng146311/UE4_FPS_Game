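; Test game mode that spawns AI bots at locations chosen by an Environment Query.
; SpawnNewBot runs BP_S_EQS in RandomBest25Pct mode and binds to its query-finished event.
; On success, each returned location gets a brief debug sphere and a spawned bot, with roughly a one-in-four chance of BP_STracker, otherwise BP_AdvancedAI.
; Nothing in this graph calls SpawnNewBot, and other query statuses are ignored.
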(event Custom|OnQueryFinishedEvent_Event_0
  (params (QueryInstance :type Env%20Query%20Instance%20Blueprint%20Wrapper%20Object%20Reference) (QueryStatus :type EEnvQueryStatus%20Enum :default "Processing"))
  (switch Utilities|FlowControl|Switch|SwitchonEEnvQueryStatus QueryStatus
    (:Success
      (for _array_element (Class|EnvQueryInstanceBlueprintWrapper|GetResultsasLocations QueryInstance)
        (Rendering|Debug|DrawDebugSphere _array_element 5e+01 12 "(R=1.000000,G=1.000000,B=1.000000,A=1.000000)" 2.0)
        (Game|SpawnActorfromClass (select (<= (Math|Random|RandomFloatinRange 0.0 1e+02) 25.0) "/Game/Blueprints/BP_STracker.BP_STracker_C" "/Game/AdvanceAI/BP_AdvancedAI.BP_AdvancedAI_C") (Math|Transform|MakeTransform _array_element) "Undefined" 0 0)))))

(event EventTick
  (params (DeltaSeconds :type Float%20%28single-precision%29)))

(event EventSpawnNewBot
  (bind _returnvalue (AI|EQS|RunEQSQuery "/Game/Blueprints/BP_S_EQS.BP_S_EQS" self "RandomBest25Pct"))
  (EventDispatchers|AssignOnQueryFinishedEvent _returnvalue (delegate Custom|OnQueryFinishedEvent_Event_0)))

(fn ConstructionScript)